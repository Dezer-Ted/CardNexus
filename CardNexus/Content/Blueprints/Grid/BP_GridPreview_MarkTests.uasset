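; Grid preview test actor whose construction script builds an X by Z grid of flattened, shadowless static mesh tiles.
; Each tile traces downward on Visibility and shows only on a hit.
; GetActorsToIgnore feeds that trace, returning at the first StaticMeshActor not named "Floor", so it ignores at most one.
; A debug-drawn upward trace also runs for visible tiles, but its hiding branch is disconnected.
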(event EventBeginPlay)

(event Collision|EventActorBeginOverlap
  (params (OtherActor :type Actor%20Object%20Reference)))

(event EventTick
  (params (DeltaSeconds :type Float%20%28single-precision%29)))

(fn ConstructionScript
  (bind _tilesize (Variables|Default|GetTileSize))
  (bind _scale (Variables|Default|GetScale))
  (for _index (range 0 (- (Variables|Default|GetXGridSize) 1))
    (for _index_2 (range 0 (- (Variables|Default|GetZGridSize) 1))
      (bind _returnvalue (AddComponent|AddStaticMeshComponent false (Math|Transform|MakeTransform (Math|Vector|MakeVector (* _index _tilesize) (* _index_2 _tilesize) 0.0) "0, 0, 0" (Math|Vector|MakeVector _scale _scale 0.1))))
      (Rendering|SetCastShadow _returnvalue false)
      (bind _actorstoignore (CallFunction|GetActorstoIgnore))
      (bind _returnvalue_2 (Collision|LineTraceByChannel (Math|Vector|MakeVector (* _index _tilesize) (* _index_2 _tilesize) 0.0) (- (Transformation|GetWorldLocation _returnvalue) "0.000000,0.000000,1000.000000") "TraceTypeQuery1" false _actorstoignore "None" true "(R=1.000000,G=0.000000,B=0.000000,A=1.000000)" "(R=0.000000,G=1.000000,B=0.000000,A=1.000000)" 1e+01))
      (if _returnvalue_2
        (Rendering|SetVisibility _returnvalue true false)
        (bind _returnvalue_3 (Collision|LineTraceByChannel (+ (Math|Vector|MakeVector (* _index _tilesize) (* _index_2 _tilesize) 0.0) "0.000000,0.000000,10.000000") (+ (Transformation|GetWorldLocation _returnvalue) "0.000000,0.000000,1000.000000") "TraceTypeQuery1" false 0 "ForDuration" true "(R=1.000000,G=0.000000,B=0.000000,A=1.000000)" "(R=0.000000,G=1.000000,B=0.000000,A=1.000000)" 1e+01))
        (else
          (Rendering|SetVisibility _returnvalue false false))))))

(fn GetActorstoIgnore
  (bind _actorstoignore (Variables|Default|GetActorsToIgnore))
  (bind _outactors (Actor|GetAllActorsOfClass "/Script/Engine.StaticMeshActor"))
  (for _array_element _outactors
    (if (not (Utilities|String|Contains (Utilities|GetDisplayName _array_element) "Floor"))
      (Utilities|Array|Add _actorstoignore _array_element)
      (return _actorstoignore)))
  (return _actorstoignore))